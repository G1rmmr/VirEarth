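; BoardActor is a touchable board that hands the player a random password in the AR game.
; A first touch on its Cube, gated by DoOnce, stores a random integer as RandomPassword on the BP_ARPawn.
; It then shows the RandomGenerationNumber widget for a few seconds, removes it and destroys itself.
; An unconnected BoardTestWidget branch never runs.
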(event OnInputTouchBegin(Cube)
  (params (FingerIndex :type ETouchIndex%20Enum :default "Touch1") (TouchedComponent :type Primitive%20Component%20Object%20Reference))
  (Utilities|FlowControl|DoOnce false
    (:Completed
      (Variables|/Game/VirEarth_YangHyeonseung/Blueprints/GameFramework/BP_ARPawn.BP_ARPawn_C|SetRandomPassword (.AsBP%20ARPawn (Utilities|Casting|CastToBP_ARPawn (Game|Player|GetPlayerPawn 0))) (Math|Random|RandomInteger 9999))
      (bind _returnvalue (UserInterface|CreateWidget "/Game/VirEarth_YangHyeonseung/Blueprints/RandomGenerationNumber.RandomGenerationNumber_C"))
      (UserInterface|Viewport|AddtoViewport _returnvalue 0)
      (Utilities|FlowControl|Delay 3.0)
      (Widget|RemovefromParent _returnvalue)
      (Actor|DestroyActor))))

(event EventBeginPlay)

(event Collision|EventActorBeginOverlap
  (params (OtherActor :type Actor%20Object%20Reference)))

(event EventTick
  (params (DeltaSeconds :type Float%20%28single-precision%29)))

(fn ConstructionScript)